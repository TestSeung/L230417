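; BP_P38 is a P-38 aircraft Blueprint that flies forward continuously and spins its two propellers.
; Each Tick offsets the actor along local X by MoveSpeed scaled by delta time, followed by a Delay that leads nowhere.
; The shared Pro function then rolls the Left and Right components at a frame-rate-independent propeller speed.
; Pitch and Roll axis events are empty, so the plane has no steering.
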(event EventTick
  (params (DeltaSeconds :type Float%20%28single-precision%29))
  (Utilities|FlowControl|Sequence
    (:then_0
      ;[1 1 1] 앞으로 이동
      (Transformation|AddActorLocalOffset (Math|Vector|MakeVector (* (Variables|속도|GetMove%20speed) (Utilities|Time|GetWorldDeltaSeconds)) 0.0 0.0) false false)
      (Utilities|FlowControl|Delay 3.0))
    (:then_1
      ;[1 1 1] 코멘트
      (CallFunction|Pro (Variables|Default|GetLeft)))
    (:then_2
      ;[1 1 1] 코멘트
      (CallFunction|Pro (Variables|Default|GetRight)))))

(event Input|AxisEvents|InputAxisPitch
  (params (AxisValue :type Float%20%28single-precision%29)))

(event Input|AxisEvents|InputAxisRoll
  (params (AxisValue :type Float%20%28single-precision%29)))

(fn ConstructionScript)

(fn Pro
  (params (where :type Static%20Mesh%20Component%20Object%20Reference))
  (Transformation|AddRelativeRotation where (Math|Rotator|MakeRotator (* (Utilities|Time|GetWorldDeltaSeconds) (Variables|Default|Get프로펠러회전속도)) 0.0 0.0) false false))